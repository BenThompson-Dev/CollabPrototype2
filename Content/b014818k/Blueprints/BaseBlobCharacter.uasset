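; Base character for a blob creature that eats food of its matching type to build progress and level up.
; Food overlaps are queried by interface; compatible food adds progress, updates the widget bar and is destroyed, with the bar visible only while the player is nearby.
; A full bar triggers an upgrade: the first enlarges the blob and raises its progress cap, the next quits the game.
; Capsule overlaps report pen entry and exit through an interface.
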(event OnComponentBeginOverlap(ProgressBarShowCollision)
  (params (OverlappedComponent :type Primitive%20Component%20Object%20Reference) (OtherActor :type Actor%20Object%20Reference) (OtherComp :type Primitive%20Component%20Object%20Reference) (OtherBodyIndex :type Integer) (bFromSweep :type Boolean) (SweepResult :type Hit%20Result%20Structure%20%28by%20ref%29))
  ;[1 1 1] b014818k - Activates and deactivates the progress bar depending if the player is close or not.
  (Utilities|Casting|CastToThirdPersonCharacter_Test OtherActor)
  (Rendering|SetVisibility (Variables|Default|GetProgressBar) true false))

(event OnComponentEndOverlap(ProgressBarShowCollision)
  (params (OverlappedComponent :type Primitive%20Component%20Object%20Reference) (OtherActor :type Actor%20Object%20Reference) (OtherComp :type Primitive%20Component%20Object%20Reference) (OtherBodyIndex :type Integer))
  ;[1 1 1] b014818k - Activates and deactivates the progress bar depending if the player is close or not.
  (Utilities|Casting|CastToThirdPersonCharacter_Test OtherActor)
  (Rendering|SetVisibility (Variables|Default|GetProgressBar) false false))

(event OnComponentBeginOverlap(CapsuleComponent)
  (params (OverlappedComponent :type Primitive%20Component%20Object%20Reference) (OtherActor :type Actor%20Object%20Reference) (OtherComp :type Primitive%20Component%20Object%20Reference) (OtherBodyIndex :type Integer) (bFromSweep :type Boolean) (SweepResult :type Hit%20Result%20Structure%20%28by%20ref%29))
  (Class|BPIBlob|IBlobinPen(Message) OtherActor (Variables|Default|GetBlobFoodType) true))

(event OnComponentBeginOverlap(FoodCollision)
  (params (OverlappedComponent :type Primitive%20Component%20Object%20Reference) (OtherActor :type Actor%20Object%20Reference) (OtherComp :type Primitive%20Component%20Object%20Reference) (OtherBodyIndex :type Integer) (bFromSweep :type Boolean) (SweepResult :type Hit%20Result%20Structure%20%28by%20ref%29))
  ;[1 1 1] b014818k - If the food type is compatible and its rarity, eat it and destroy if can.
  (bind _foodreference (Class|BPIBlob|IGetFood(Message) OtherActor))
  (bind _output_get (Variables|Default|SetBlobProgressGainFromFood (Variables|/Game/b014818k/Blueprints/Food.Food_C|GetBlobFeedAmount _foodreference)))
  (if (Utilities|Enum|Equal(Enum) (Variables|/Game/b014818k/Blueprints/Food.Food_C|GetFoodType _foodreference) (Variables|Default|GetBlobFoodType))
    (CallFunction|BlobFed _output_get)
    (Actor|DestroyActor _foodreference)
    (else
      (Development|PrintString "Cant eat"))))

(event OnComponentEndOverlap(CapsuleComponent)
  (params (OverlappedComponent :type Primitive%20Component%20Object%20Reference) (OtherActor :type Actor%20Object%20Reference) (OtherComp :type Primitive%20Component%20Object%20Reference) (OtherBodyIndex :type Integer))
  (Class|BPIBlob|IBlobinPen(Message) OtherActor (Variables|Default|GetBlobFoodType) false))

(event Custom|BlobFed
  (params (FeedAmount :type Float%20%28single-precision%29))
  ;[1 1 1] b014818k - Call update UI function, check if blob reached max progress.
  (CallFunction|UpdateProgressUI FeedAmount)
  (if (<= (Variables|Default|GetBlobMaxProgress) (Variables|Default|GetBlobCurrentProgress))
    (CallFunction|Upgrade)))

(event EventBeginPlay
  (Rendering|SetVisibility (Variables|Default|GetProgressBar) false false))

(fn ConstructionScript)

(fn UpdateProgressUI
  (params (Progress :type Float%20%28single-precision%29))
  (Class|BPIBlob|IUpdateBlobProgressBar(Message) (UserInterface|GetUserWidgetObject (Variables|Default|GetProgressBar)) (+ Progress (Variables|Default|GetBlobCurrentProgress)) (Variables|Default|GetBlobMaxProgress))
  (Variables|Default|SetBlobCurrentProgress (+ Progress (Variables|Default|GetBlobCurrentProgress))))

(fn Upgrade
  ;[1 1 1] b014818k - Upgrades the blob to the next stage
  (if (== (Variables|Default|GetBlobLevel) 0)
    (Development|PrintString "Level 2")
    (Transformation|SetActorScale3D (* (Transformation|GetActorScale3D) 1.5))
    (Variables|Default|SetBlobMaxProgress (* 1.5 (Variables|Default|GetBlobMaxProgress)))
    (Variables|Default|SetMapProgressGain (* 1.5 (Variables|Default|GetMapProgressGain)))
    (bind _output_get (Variables|Default|SetBlobCurrentProgress 0.0))
    (CallFunction|UpdateProgressUI _output_get)
    (Variables|Default|SetBlobLevel 1)
    (else
      (Development|PrintString "Level 3")
      (Game|QuitGame 0 "Quit" false))))

(fn ICheckFoodType
  (return "NewEnumerator0" 0.0))

(fn IGetFood)