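; Base blob that eats food of a matching type to build progress toward upgrades.
; Its feed collision checks food through an interface, destroys matches, and pushes new progress to the widget via another interface.
; When progress exactly equals the maximum, it scales the maximum and light progress gain without resetting progress.
; A second collision shows the progress bar only while the player character overlaps it.
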(event OnComponentBeginOverlap(ProgressBarCollision)
  (params (OverlappedComponent :type Primitive%20Component%20Object%20Reference) (OtherActor :type Actor%20Object%20Reference) (OtherComp :type Primitive%20Component%20Object%20Reference) (OtherBodyIndex :type Integer) (bFromSweep :type Boolean) (SweepResult :type Hit%20Result%20Structure%20%28by%20ref%29))
  ;[1 1 1] b014818k - Activates and deactivates the progress bar depending if the player is close or not.
  (Utilities|Casting|CastToThirdPersonCharacter_Test OtherActor)
  (Rendering|SetVisibility (Variables|Default|GetProgressBar) true false))

(event OnComponentEndOverlap(ProgressBarCollision)
  (params (OverlappedComponent :type Primitive%20Component%20Object%20Reference) (OtherActor :type Actor%20Object%20Reference) (OtherComp :type Primitive%20Component%20Object%20Reference) (OtherBodyIndex :type Integer))
  ;[1 1 1] b014818k - Activates and deactivates the progress bar depending if the player is close or not.
  (Utilities|Casting|CastToThirdPersonCharacter_Test OtherActor)
  (Rendering|SetVisibility (Variables|Default|GetProgressBar) false false))

(event OnComponentBeginOverlap(FeedCollision)
  (params (OverlappedComponent :type Primitive%20Component%20Object%20Reference) (OtherActor :type Actor%20Object%20Reference) (OtherComp :type Primitive%20Component%20Object%20Reference) (OtherBodyIndex :type Integer) (bFromSweep :type Boolean) (SweepResult :type Hit%20Result%20Structure%20%28by%20ref%29))
  ;[1 1 1] b014818k - If the food type is compatible, eat it and destroy.
  (bind _foodtype (Class|BPIBlob|ICheckFoodType(Message) OtherActor))
  (if (Utilities|Enum|Equal(Enum) _foodtype (Variables|Default|GetBlobFoodType))
    (CallFunction|BlobFed (Variables|Default|GetBlobProgressGainFromFood))
    (Actor|DestroyActor OtherActor)
    (else
      (Development|PrintString "Cant eat"))))

(event Custom|BlobFed
  (params (FeedAmount :type Float%20%28single-precision%29))
  ;[1 1 1] b014818k - Call update UI function, check if blob reached max progress.
  (CallFunction|UpdateProgressUI FeedAmount)
  (if (== (Variables|Default|GetBlobMaxProgress) (Variables|Default|GetBlobCurrentProgress))
    (CallFunction|Upgrade)))

(event EventBeginPlay
  (Rendering|SetVisibility (Variables|Default|GetProgressBar) false false))

(fn ConstructionScript)

(fn UpdateProgressUI
  (params (Progress :type Float%20%28single-precision%29))
  (Class|BPIBlob|IUpdateBlobProgressBar(Message) (UserInterface|GetUserWidgetObject (Variables|Default|GetProgressBar)) (+ Progress (Variables|Default|GetBlobCurrentProgress)))
  (Variables|Default|SetBlobCurrentProgress (+ Progress (Variables|Default|GetBlobCurrentProgress))))

(fn Upgrade
  ;[1 1 1] b014818k - Upgrades the blob to the next stage
  (Variables|Default|SetBlobMaxProgress (* 1.5 (Variables|Default|GetBlobMaxProgress)))
  (Variables|Default|SetLightProgressGain (* 1.5 (Variables|Default|GetLightProgressGain)))
  (Development|PrintString "Upgraded"))

(fn ICheckFoodType
  (return "NewEnumerator0" "NewEnumerator0"))