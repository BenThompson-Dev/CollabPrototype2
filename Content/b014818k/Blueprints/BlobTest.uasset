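; BlobTest is a test blob actor that shows a progress widget when the player's test character is nearby.
; A looping timer started on BeginPlay casts the widget component's user widget to W_BlobProgress and periodically increments its BlobProgress value, regardless of visibility.
; The widget starts hidden, and Sphere1 overlap begin and end events toggle its visibility for ThirdPersonCharacter_Test only.
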(event OnComponentBeginOverlap(Sphere1)
  (params (OverlappedComponent :type Primitive%20Component%20Object%20Reference) (OtherActor :type Actor%20Object%20Reference) (OtherComp :type Primitive%20Component%20Object%20Reference) (OtherBodyIndex :type Integer) (bFromSweep :type Boolean) (SweepResult :type Hit%20Result%20Structure%20%28by%20ref%29))
  (Utilities|Casting|CastToThirdPersonCharacter_Test OtherActor)
  (Rendering|SetVisibility (Variables|Default|GetWidget) true false))

(event OnComponentEndOverlap(Sphere1)
  (params (OverlappedComponent :type Primitive%20Component%20Object%20Reference) (OtherActor :type Actor%20Object%20Reference) (OtherComp :type Primitive%20Component%20Object%20Reference) (OtherBodyIndex :type Integer))
  (Utilities|Casting|CastToThirdPersonCharacter_Test OtherActor)
  (Rendering|SetVisibility (Variables|Default|GetWidget) false false))

(event Custom|CustomEvent_0
  (bind _asw_blob_progress (Utilities|Casting|CastToW_BlobProgress (UserInterface|GetUserWidgetObject (Variables|Default|GetWidget))))
  (Variables|/Game/b014818k/UI/W_BlobProgress.W_BlobProgress_C|SetBlobProgress _asw_blob_progress (+ (Variables|/Game/b014818k/UI/W_BlobProgress.W_BlobProgress_C|GetBlobProgress _asw_blob_progress) 1e+01)))

(event EventBeginPlay
  (Rendering|SetVisibility (Variables|Default|GetWidget) false false)
  (Utilities|Time|SetTimerbyEvent (delegate Custom|CustomEvent_0) 2.0 true))

(fn ConstructionScript)