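; Food actor Blueprint that carries a food type and a randomly rolled rarity.
; On BeginPlay, chained weighted random booleans pick one of four FoodRarity enum values, giving each tier different odds.
; The I_CheckFoodType interface function returns FoodType and FoodRarity to callers; FoodType is never assigned in these graphs.
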(event EventBeginPlay
  (if (Math|Random|RandomBoolwithWeight 0.5)
    (Variables|Default|SetFoodRarity "NewEnumerator1")
    (elif (Math|Random|RandomBoolwithWeight 0.4)
      (Variables|Default|SetFoodRarity "NewEnumerator0")
      (elif (Math|Random|RandomBoolwithWeight 0.6)
        (Variables|Default|SetFoodRarity "NewEnumerator2")
        (else
          (Variables|Default|SetFoodRarity "NewEnumerator3"))))))

(fn ConstructionScript)

(fn ICheckFoodType
  (return (Variables|Default|GetFoodType) (Variables|Default|GetFoodRarity)))