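; Blocking wall actor that toggles a barrier based on the CreatureEvolved flag.
; On BeginPlay only, a true flag shows the wall with query and physics collision, while false hides it and disables collision.
; This runs opposite to the graph comment about removing walls after evolution, and the "True"/"False" debug prints are also inverted relative to the flag.
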(event Collision|EventActorBeginOverlap
  (params (OtherActor :type Actor%20Object%20Reference)))

(event EventTick
  (params (DeltaSeconds :type Float%20%28single-precision%29)))

(event EventBeginPlay
  ;[1 1 1] Check if a creature has evolved and remove the walls
  (if (Variables|Default|GetCreature%20Evolved)
    (Rendering|SetVisibility (Variables|Default|Get%20%20) true false)
    (Collision|SetCollisionEnabled (Variables|Default|Get%20%20) "QueryAndPhysics")
    (Development|PrintString "False")
    (else
      (Rendering|SetVisibility (Variables|Default|Get%20%20) false false)
      (Collision|SetCollisionEnabled (Variables|Default|GetTarget) "NoCollision")
      (Development|PrintString "True"))))

(fn ConstructionScript)