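; Inventory component that stores its owner's items as an array of slot structs, each with a name, sprite and count.
; Adding an item stacks onto an entry with the same name or appends a new one, matching by name so differing counts don't create duplicates.
; Replacing an item removes it at zero count.
; Add, replace and remove push changes to the owner's UI through interface messages, while use only decrements the count.
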(fn GetInventoryItem
  (params (itemIndex :type Integer))
  (return (Utilities|Array|Get(acopy) (Variables|Default|GetinventorySlots) itemIndex)))

(fn AddInventoryItem
  (params (itemToAdd :type STR%20Inventory%20Item%20Structure))
  (bind (_isinarray _arrayindex) (CallFunction|FindItemIndex itemToAdd)) ; Looks to see if the item is already\nin the player's inventory
  (if _isinarray ; Checks to see if the item\nis already contained in the array
    ;[1 1 1] Finds the item's stored position in the array and adds the correct amount to it
    (bind _output_get (LocalVariables|SetnewItemIndex _arrayindex))
    (Utilities|Array|SetArrayElem (Variables|Default|GetinventorySlots) (LocalVariables|GetnewItemIndex) (Utilities|Struct|MakeSTR_InventoryItem (.itemName (Utilities|Struct|BreakSTR_InventoryItem (Utilities|Array|Get(acopy) (Variables|Default|GetinventorySlots) _output_get))) (.itemSprite (Utilities|Struct|BreakSTR_InventoryItem (Utilities|Array|Get(acopy) (Variables|Default|GetinventorySlots) _output_get))) (+ (.itemCount (Utilities|Struct|BreakSTR_InventoryItem (Utilities|Array|Get(acopy) (Variables|Default|GetinventorySlots) _output_get))) (.itemCount (Utilities|Struct|BreakSTR_InventoryItem itemToAdd)))))
    (else
      ;[1 1 1] Handles adding a new item element into the array
      (bind _returnvalue (Utilities|Array|AddUnique (Variables|Default|GetinventorySlots) itemToAdd)) ; Adds the item into the array
      (LocalVariables|SetnewItemIndex _returnvalue)))
  ;[1 1 1] Updates the inventory UI
  (bind _inventorywidget (Class|BPIPlayer|IGetUI(Message) (Components|GetOwner)))
  (Class|BPIUI|ISetInventoryUI(Message) _inventorywidget (Utilities|Array|Get(acopy) (Variables|Default|GetinventorySlots) (LocalVariables|GetnewItemIndex)) (LocalVariables|GetnewItemIndex)))

(fn UseInventoryItem
  (params (itemIndex :type Integer))
  (Math|Integer|DecrementInt (.itemCount (Utilities|Struct|BreakSTR_InventoryItem (Utilities|Array|Get(acopy) (Variables|Default|GetinventorySlots) itemIndex)))))

(fn FindItemIndex
  (params (item :type STR%20Inventory%20Item%20Structure))
  ;[1 1 1] Goes through each element in the inventory to see if it already is in the inventory by comparing names, if full structs were compared then the count values would result in multiple entries
  (if (!= (Utilities|Array|Length (Variables|Default|GetinventorySlots)) 0) ; Checks to make sure the array\ndoesn't have a length of 0
    (bind (_array_element _array_index) (Utilities|Array|ForEachLoopwithBreak (Variables|Default|GetinventorySlots) :!label _label)
      (:LoopBody
        (if (Utilities|Enum|Equal(Enum) (.itemName (Utilities|Struct|BreakSTR_InventoryItem _array_element)) (.itemName (Utilities|Struct|BreakSTR_InventoryItem item)))
          (LocalVariables|SethasItemBeenFound true)
          (LocalVariables|SetfoundItemIndex _array_index)
          (goto _label Break)))
      (:Completed
        (return (LocalVariables|GethasItemBeenFound) (LocalVariables|GetfoundItemIndex))))
    (else
      (return (LocalVariables|GethasItemBeenFound) (LocalVariables|GetfoundItemIndex)))))

(fn FindItem
  (params (itemToFind :type STR%20Inventory%20Item%20Structure))
  ;[1 1 1] Finds and returns a reference to the item
  (bind (_isinarray _arrayindex) (CallFunction|FindItemIndex itemToFind))
  (if _isinarray
    (bind _inventoryitem (CallFunction|GetInventoryItem _arrayindex))
    (return _inventoryitem)))

(fn ReplaceItem
  (params (updatedItem :type STR%20Inventory%20Item%20Structure))
  (bind (_isinarray _arrayindex) (CallFunction|FindItemIndex updatedItem))
  (if _isinarray
    (if (<= (.itemCount (Utilities|Struct|BreakSTR_InventoryItem updatedItem)) 0)
      (CallFunction|RemoveInventoryItem _arrayindex)
      (else
        (Utilities|Array|SetArrayElem (Variables|Default|GetinventorySlots) _arrayindex updatedItem)))
    (bind _inventorywidget (Class|BPIPlayer|IGetUI(Message) (Components|GetOwner)))
    (Class|BPIUI|ISetInventoryUI(Message) _inventorywidget (Utilities|Array|Get(acopy) (Variables|Default|GetinventorySlots) _arrayindex) _arrayindex)))

(fn RemoveInventoryItem
  (params (arrayIndex :type Integer))
  (Utilities|Array|RemoveIndex (Variables|Default|GetinventorySlots) arrayIndex)
  ;[1 1 1] Updates all the UI elements
  (bind _inventorywidget (Class|BPIPlayer|IGetUI(Message) (Components|GetOwner)))
  (Class|BPIUI|IUpdateAllUIs(Message) _inventorywidget (Variables|Default|GetinventorySlots)))